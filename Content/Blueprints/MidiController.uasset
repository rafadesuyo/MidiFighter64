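; Actor that mirrors a 32-button MIDI Fighter-style controller, playing sounds and lighting its circle meshes from MIDI input.
; Construction script creates a dynamic material per circle; BeginPlay opens hardcoded MIDI device 1 and binds note and pitch-bend events.
; Note-on for notes 53–84 plays a sound at world origin and sets that circle's emission color; note-off blacks it out.
; Pitch bend and key 1 (device ID listing) print debug text.
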(event `MidiPitch`
  (params (MIDIDeviceController :type "MIDIDeviceInputController Object Reference") (Timestamp :type Integer) (Channel :type Integer) (Pitch :type Integer))
  (`KismetSystemLibrary.PrintString` (`KismetStringLibrary.Concat_StrStr` "Pitch " (`KismetStringLibrary.Conv_IntToString` Pitch)) true true (struct :`R` 0.351149 :`G` 1.0 :`B` 0.541507 :`A` 1.0)))

(event `Key|One`
  (params (Key :type "Key Structure"))
  (:`Pressed`
    (bind _outmididevices (`MIDIDeviceManager.FindMIDIDevices`))
    (for _array_element _outmididevices
      (`KismetSystemLibrary.PrintString` (`KismetStringLibrary.Conv_IntToString` (`.DeviceID` (break `FoundMIDIDevice` _array_element))) true true (struct :`G` 0.66 :`B` 1.0 :`A` 1.0) 5.0))))

(event `self.ReceiveBeginPlay`
  (bind _returnvalue (`MIDIDeviceManager.CreateMIDIDeviceInputController` 1))
  (bind _output_get (set `self.MidiController` _returnvalue))
  (add `MIDIDeviceInputController.OnMIDINoteOn` _output_get (`|CreateDelegate` :!event `MidiButtonOn`))
  (add `MIDIDeviceInputController.OnMIDIPitchBend` _output_get (`|CreateDelegate` :!event `MidiPitch`))
  (add `MIDIDeviceInputController.OnMIDINoteOff` _output_get (`|CreateDelegate` :!event `MidiButtonOff`)))

(event `MidiButtonOff`
  (params (MIDIDeviceController :type "MIDIDeviceInputController Object Reference") (Timestamp :type Integer) (Channel :type Integer) (Note :type Integer) (Velocity :type Integer))
  (switch `int` Note
    (:`53`
      (`MaterialInstanceDynamic.SetVectorParameterValue` (`self.DynamicMaterial01`) "EmissionColor" (struct :`A` 1.0)))
    (:`54`
      (`MaterialInstanceDynamic.SetVectorParameterValue` (`self.DynamicMaterial02`) "EmissionColor" (struct :`A` 1.0)))
    (:`55`
      (`MaterialInstanceDynamic.SetVectorParameterValue` (`self.DynamicMaterial03`) "EmissionColor" (struct :`A` 1.0)))
    (:`56`
      (`MaterialInstanceDynamic.SetVectorParameterValue` (`self.DynamicMaterial04`) "EmissionColor" (struct :`A` 1.0)))
    (:`57`
      (`MaterialInstanceDynamic.SetVectorParameterValue` (`self.DynamicMaterial05`) "EmissionColor" (struct :`A` 1.0)))
    (:`58`
      (`MaterialInstanceDynamic.SetVectorParameterValue` (`self.DynamicMaterial06`) "EmissionColor" (struct :`A` 1.0)))
    (:`59`
      (`MaterialInstanceDynamic.SetVectorParameterValue` (`self.07`) "EmissionColor" (struct :`A` 1.0)))
    (:`60`
      (`MaterialInstanceDynamic.SetVectorParameterValue` (`self.08`) "EmissionColor" (struct :`A` 1.0)))
    (:`61`
      (`MaterialInstanceDynamic.SetVectorParameterValue` (`self.09`) "EmissionColor" (struct :`A` 1.0)))
    (:`62`
      (`MaterialInstanceDynamic.SetVectorParameterValue` (`self.10`) "EmissionColor" (struct :`A` 1.0)))
    (:`63`
      (`MaterialInstanceDynamic.SetVectorParameterValue` (`self.11`) "EmissionColor" (struct :`A` 1.0)))
    (:`64`
      (`MaterialInstanceDynamic.SetVectorParameterValue` (`self.12`) "EmissionColor" (struct :`A` 1.0)))
    (:`65`
      (`MaterialInstanceDynamic.SetVectorParameterValue` (`self.13`) "EmissionColor" (struct :`A` 1.0)))
    (:`66`
      (`MaterialInstanceDynamic.SetVectorParameterValue` (`self.14`) "EmissionColor" (struct :`A` 1.0)))
    (:`67`
      (`MaterialInstanceDynamic.SetVectorParameterValue` (`self.15`) "EmissionColor" (struct :`A` 1.0)))
    (:`68`
      (`MaterialInstanceDynamic.SetVectorParameterValue` (`self.16`) "EmissionColor" (struct :`A` 1.0)))
    (:`69`
      (`MaterialInstanceDynamic.SetVectorParameterValue` (`self.17`) "EmissionColor" (struct :`A` 1.0)))
    (:`70`
      (`MaterialInstanceDynamic.SetVectorParameterValue` (`self.18`) "EmissionColor" (struct :`A` 1.0)))
    (:`71`
      (`MaterialInstanceDynamic.SetVectorParameterValue` (`self.19`) "EmissionColor" (struct :`A` 1.0)))
    (:`72`
      (`MaterialInstanceDynamic.SetVectorParameterValue` (`self.20`) "EmissionColor" (struct :`A` 1.0)))
    (:`73`
      (`MaterialInstanceDynamic.SetVectorParameterValue` (`self.21`) "EmissionColor" (struct :`A` 1.0)))
    (:`74`
      (`MaterialInstanceDynamic.SetVectorParameterValue` (`self.22`) "EmissionColor" (struct :`A` 1.0)))
    (:`75`
      (`MaterialInstanceDynamic.SetVectorParameterValue` (`self.23`) "EmissionColor" (struct :`A` 1.0)))
    (:`76`
      (`MaterialInstanceDynamic.SetVectorParameterValue` (`self.24`) "EmissionColor" (struct :`A` 1.0)))
    (:`77`
      (`MaterialInstanceDynamic.SetVectorParameterValue` (`self.25`) "EmissionColor" (struct :`A` 1.0)))
    (:`78`
      (`MaterialInstanceDynamic.SetVectorParameterValue` (`self.26`) "EmissionColor" (struct :`A` 1.0)))
    (:`79`
      (`MaterialInstanceDynamic.SetVectorParameterValue` (`self.27`) "EmissionColor" (struct :`A` 1.0)))
    (:`80`
      (`MaterialInstanceDynamic.SetVectorParameterValue` (`self.28`) "EmissionColor" (struct :`A` 1.0)))
    (:`81`
      (`MaterialInstanceDynamic.SetVectorParameterValue` (`self.29`) "EmissionColor" (struct :`A` 1.0)))
    (:`82`
      (`MaterialInstanceDynamic.SetVectorParameterValue` (`self.30`) "EmissionColor" (struct :`A` 1.0)))
    (:`83`
      (`MaterialInstanceDynamic.SetVectorParameterValue` (`self.31`) "EmissionColor" (struct :`A` 1.0)))
    (:`84`
      (`MaterialInstanceDynamic.SetVectorParameterValue` (`self.32`) "EmissionColor" (struct :`A` 1.0)))))

(event `MidiButtonOn`
  (params (MIDIDeviceController :type "MIDIDeviceInputController Object Reference") (Timestamp :type Integer) (Channel :type Integer) (Note :type Integer) (Velocity :type Integer))
  (switch `int` Note
    (:`53`
      (`GameplayStatics.PlaySoundAtLocation` "/Game/Audio/01.01" (0.0 0.0 0.0) (struct) 1.0 1.0 0.0 null null null null)
      (`MaterialInstanceDynamic.SetVectorParameterValue` (`self.DynamicMaterial01`) "EmissionColor" (struct :`R` 0.093059 :`G` 0.701102 :`B` 0.114435 :`A` 1.0)))
    (:`54`
      (`GameplayStatics.PlaySoundAtLocation` "/Game/Audio/02.02" (0.0 0.0 0.0) (struct) 1.0 1.0 0.0 null null null null)
      (`MaterialInstanceDynamic.SetVectorParameterValue` (`self.DynamicMaterial02`) "EmissionColor" (struct :`R` 0.658375 :`G` 0.007499 :`B` 0.3564 :`A` 1.0)))
    (:`55`
      (`GameplayStatics.PlaySoundAtLocation` "/Game/Audio/06.06" (0.0 0.0 0.0) (struct) 1.0 1.0 0.0 null null null null)
      (`MaterialInstanceDynamic.SetVectorParameterValue` (`self.DynamicMaterial03`) "EmissionColor" (struct :`R` 0.219011 :`G` 0.12693 :`B` 0.658375 :`A` 1.0)))
    (:`56`
      (`GameplayStatics.PlaySoundAtLocation` "/Game/Audio/08.08" (0.0 0.0 0.0) (struct) 1.0 1.0 0.0 null null null null)
      (`MaterialInstanceDynamic.SetVectorParameterValue` (`self.DynamicMaterial04`) "EmissionColor" (struct :`R` 0.042369 :`G` 0.53969 :`B` 0.658375 :`A` 1.0)))
    (:`57`
      (`GameplayStatics.PlaySoundAtLocation` "/Game/Audio/13.13" (0.0 0.0 0.0) (struct) 1.0 1.0 0.0 null null null null)
      (`MaterialInstanceDynamic.SetVectorParameterValue` (`self.DynamicMaterial05`) "EmissionColor" (struct :`R` 0.068581 :`G` 0.658375 :`B` 0.143347 :`A` 1.0)))
    (:`58`
      (`GameplayStatics.PlaySoundAtLocation` "/Game/Audio/19.19" (0.0 0.0 0.0) (struct) 1.0 1.0 0.0 null null null null)
      (`MaterialInstanceDynamic.SetVectorParameterValue` (`self.DynamicMaterial06`) "EmissionColor" (struct :`R` 0.658375 :`G` 0.091141 :`B` 0.230192 :`A` 1.0)))
    (:`59`
      (`GameplayStatics.PlaySoundAtLocation` "/Game/Audio/32.32" (0.0 0.0 0.0) (struct) 1.0 1.0 0.0 null null null null)
      (`MaterialInstanceDynamic.SetVectorParameterValue` (`self.07`) "EmissionColor" (struct :`R` 0.658375 :`G` 0.550196 :`B` 0.114465 :`A` 1.0)))
    (:`60`
      (`GameplayStatics.PlaySoundAtLocation` "/Game/Audio/29.29" (0.0 0.0 0.0) (struct) 1.0 1.0 0.0 null null null null)
      (`MaterialInstanceDynamic.SetVectorParameterValue` (`self.08`) "EmissionColor" (struct :`R` 0.155439 :`G` 0.658375 :`B` 0.406907 :`A` 1.0)))
    (:`61`
      (`GameplayStatics.PlaySoundAtLocation` "/Game/Audio/07.07" (0.0 0.0 0.0) (struct) 1.0 1.0 0.0 null null null null)
      (`MaterialInstanceDynamic.SetVectorParameterValue` (`self.09`) "EmissionColor" (struct :`R` 0.270645 :`G` 0.658375 :`B` 0.134416 :`A` 1.0)))
    (:`62`
      (`GameplayStatics.PlaySoundAtLocation` "/Game/Audio/12.12" (0.0 0.0 0.0) (struct) 1.0 1.0 0.0 null null null null)
      (`MaterialInstanceDynamic.SetVectorParameterValue` (`self.10`) "EmissionColor" (struct :`G` 0.658375 :`B` 0.398005 :`A` 1.0)))
    (:`63`
      (`GameplayStatics.PlaySoundAtLocation` "/Game/Audio/03.03" (0.0 0.0 0.0) (struct) 1.0 1.0 0.0 null null null null)
      (`MaterialInstanceDynamic.SetVectorParameterValue` (`self.11`) "EmissionColor" (struct :`G` 0.658375 :`B` 0.398005 :`A` 1.0)))
    (:`64`
      (`GameplayStatics.PlaySoundAtLocation` "/Game/Audio/31.31" (0.0 0.0 0.0) (struct) 1.0 1.0 0.0 null null null null)
      (`MaterialInstanceDynamic.SetVectorParameterValue` (`self.12`) "EmissionColor" (struct :`R` 0.366907 :`G` 0.075439 :`B` 0.658375 :`A` 1.0)))
    (:`65`
      (`GameplayStatics.PlaySoundAtLocation` "/Game/Audio/14.14" (0.0 0.0 0.0) (struct) 1.0 1.0 0.0 null null null null)
      (`MaterialInstanceDynamic.SetVectorParameterValue` (`self.13`) "EmissionColor" (struct :`R` 0.658375 :`B` 0.326388 :`A` 1.0)))
    (:`66`
      (`GameplayStatics.PlaySoundAtLocation` "/Game/Audio/20.20" (0.0 0.0 0.0) (struct) 1.0 1.0 0.0 null null null null)
      (`MaterialInstanceDynamic.SetVectorParameterValue` (`self.14`) "EmissionColor" (struct :`R` 0.289851 :`G` 0.132445 :`B` 0.658375 :`A` 1.0)))
    (:`67`
      (`GameplayStatics.PlaySoundAtLocation` "/Game/Audio/25.25" (0.0 0.0 0.0) (struct) 1.0 1.0 0.0 null null null null)
      (`MaterialInstanceDynamic.SetVectorParameterValue` (`self.15`) "EmissionColor" (struct :`R` 0.658375 :`G` 0.109729 :`B` 0.283701 :`A` 1.0)))
    (:`68`
      (`GameplayStatics.PlaySoundAtLocation` "/Game/Audio/30.30" (0.0 0.0 0.0) (struct) 1.0 1.0 0.0 null null null null)
      (`MaterialInstanceDynamic.SetVectorParameterValue` (`self.16`) "EmissionColor" (struct :`R` 0.306481 :`G` 0.658375 :`B` 0.165929 :`A` 1.0)))
    (:`69`
      (`GameplayStatics.PlaySoundAtLocation` "/Game/Audio/04.04" (0.0 0.0 0.0) (struct) 1.0 1.0 0.0 null null null null)
      (`MaterialInstanceDynamic.SetVectorParameterValue` (`self.17`) "EmissionColor" (struct :`R` 0.080911 :`G` 0.658375 :`B` 0.299595 :`A` 1.0)))
    (:`70`
      (`GameplayStatics.PlaySoundAtLocation` "/Game/Audio/28.28" (0.0 0.0 0.0) (struct) 1.0 1.0 0.0 null null null null)
      (`MaterialInstanceDynamic.SetVectorParameterValue` (`self.18`) "EmissionColor" (struct :`R` 0.658375 :`G` 0.227906 :`B` 0.048007 :`A` 1.0)))
    (:`71`
      (`GameplayStatics.PlaySoundAtLocation` "/Game/Audio/15.15" (0.0 0.0 0.0) (struct) 1.0 1.0 0.0 null null null null)
      (`MaterialInstanceDynamic.SetVectorParameterValue` (`self.19`) "EmissionColor" (struct :`R` 0.123445 :`G` 0.13584 :`B` 0.658375 :`A` 1.0)))
    (:`72`
      (`GameplayStatics.PlaySoundAtLocation` "/Game/Audio/05.05" (0.0 0.0 0.0) (struct) 1.0 1.0 0.0 null null null null)
      (`MaterialInstanceDynamic.SetVectorParameterValue` (`self.20`) "EmissionColor" (struct :`R` 0.181998 :`G` 0.41815 :`B` 0.658375 :`A` 1.0)))
    (:`73`
      (`GameplayStatics.PlaySoundAtLocation` "/Game/Audio/09.09" (0.0 0.0 0.0) (struct) 1.0 1.0 0.0 null null null null)
      (`MaterialInstanceDynamic.SetVectorParameterValue` (`self.21`) "EmissionColor" (struct :`R` 0.658375 :`G` 0.192733 :`B` 0.551227 :`A` 1.0)))
    (:`74`
      (`GameplayStatics.PlaySoundAtLocation` "/Game/Audio/23.23" (0.0 0.0 0.0) (struct) 1.0 1.0 0.0 null null null null)
      (`MaterialInstanceDynamic.SetVectorParameterValue` (`self.22`) "EmissionColor" (struct :`R` 0.658375 :`G` 0.534716 :`B` 0.163737 :`A` 1.0)))
    (:`75`
      (`GameplayStatics.PlaySoundAtLocation` "/Game/Audio/10.10" (0.0 0.0 0.0) (struct) 1.0 1.0 0.0 null null null null)
      (`MaterialInstanceDynamic.SetVectorParameterValue` (`self.23`) "EmissionColor" (struct :`R` 0.658375 :`G` 0.139866 :`B` 0.093968 :`A` 1.0)))
    (:`76`
      (`GameplayStatics.PlaySoundAtLocation` "/Game/Audio/11.11" (0.0 0.0 0.0) (struct) 1.0 1.0 0.0 null null null null)
      (`MaterialInstanceDynamic.SetVectorParameterValue` (`self.24`) "EmissionColor" (struct :`R` 0.311313 :`G` 0.35629 :`B` 0.658375 :`A` 1.0)))
    (:`77`
      (`GameplayStatics.PlaySoundAtLocation` "/Game/Audio/16.16" (0.0 0.0 0.0) (struct) 1.0 1.0 0.0 null null null null)
      (`MaterialInstanceDynamic.SetVectorParameterValue` (`self.25`) "EmissionColor" (struct :`R` 0.17068 :`G` 0.658375 :`B` 0.448305 :`A` 1.0)))
    (:`78`
      (`GameplayStatics.PlaySoundAtLocation` "/Game/Audio/18.18" (0.0 0.0 0.0) (struct) 1.0 1.0 0.0 null null null null)
      (`MaterialInstanceDynamic.SetVectorParameterValue` (`self.26`) "EmissionColor" (struct :`R` 0.658375 :`G` 0.112436 :`B` 0.35708 :`A` 1.0)))
    (:`79`
      (`GameplayStatics.PlaySoundAtLocation` "/Game/Audio/21.21" (0.0 0.0 0.0) (struct) 1.0 1.0 0.0 null null null null)
      (`MaterialInstanceDynamic.SetVectorParameterValue` (`self.27`) "EmissionColor" (struct :`R` 0.204245 :`G` 0.658375 :`A` 1.0)))
    (:`80`
      (`GameplayStatics.PlaySoundAtLocation` "/Game/Audio/24.24" (0.0 0.0 0.0) (struct) 1.0 1.0 0.0 null null null null)
      (`MaterialInstanceDynamic.SetVectorParameterValue` (`self.28`) "EmissionColor" (struct :`R` 0.085726 :`G` 0.026092 :`B` 0.658375 :`A` 1.0)))
    (:`81`
      (`GameplayStatics.PlaySoundAtLocation` "/Game/Audio/17.17" (0.0 0.0 0.0) (struct) 1.0 1.0 0.0 null null null null)
      (`MaterialInstanceDynamic.SetVectorParameterValue` (`self.29`) "EmissionColor" (struct :`R` 0.658375 :`B` 0.170679 :`A` 1.0)))
    (:`82`
      (`GameplayStatics.PlaySoundAtLocation` "/Game/Audio/26.26" (0.0 0.0 0.0) (struct) 1.0 1.0 0.0 null null null null)
      (`MaterialInstanceDynamic.SetVectorParameterValue` (`self.30`) "EmissionColor" (struct :`R` 0.658375 :`G` 0.302106 :`A` 1.0)))
    (:`83`
      (`GameplayStatics.PlaySoundAtLocation` "/Game/Audio/22.22" (0.0 0.0 0.0) (struct) 1.0 1.0 0.0 null null null null)
      (`MaterialInstanceDynamic.SetVectorParameterValue` (`self.31`) "EmissionColor" (struct :`G` 0.109031 :`B` 0.658375 :`A` 1.0)))
    (:`84`
      (`GameplayStatics.PlaySoundAtLocation` "/Game/Audio/27.27" (0.0 0.0 0.0) (struct) 1.0 1.0 0.0 null null null null)
      (`MaterialInstanceDynamic.SetVectorParameterValue` (`self.32`) "EmissionColor" (struct :`R` 0.658375 :`B` 0.346826 :`A` 1.0)))))

(fn `UserConstructionScript`
  (`|ExecutionSequence`
    (:`then_0`
      (bind _returnvalue (`PrimitiveComponent.CreateDynamicMaterialInstance` (`self.MidiFighter_Circle_005`) 1 null "None"))
      (set `self.DynamicMaterial01` _returnvalue))
    (:`then_1`
      (bind _returnvalue_2 (`PrimitiveComponent.CreateDynamicMaterialInstance` (`self.MidiFighter_Circle_058`) 1 null "None"))
      (set `self.DynamicMaterial02` _returnvalue_2))
    (:`then_2`
      (bind _returnvalue_3 (`PrimitiveComponent.CreateDynamicMaterialInstance` (`self.MidiFighter_Circle_028`) 1 null "None"))
      (set `self.DynamicMaterial03` _returnvalue_3))
    (:`then_3`
      (bind _returnvalue_4 (`PrimitiveComponent.CreateDynamicMaterialInstance` (`self.MidiFighter_Circle_027`) 1 null "None"))
      (set `self.DynamicMaterial04` _returnvalue_4))
    (:`then_4`
      (bind _returnvalue_5 (`PrimitiveComponent.CreateDynamicMaterialInstance` (`self.MidiFighter_Circle_024`) 1 null "None"))
      (set `self.DynamicMaterial05` _returnvalue_5))
    (:`then_5`
      (bind _returnvalue_6 (`PrimitiveComponent.CreateDynamicMaterialInstance` (`self.MidiFighter_Circle_036`) 1 null "None"))
      (set `self.DynamicMaterial06` _returnvalue_6))
    (:`then_6`
      (bind _returnvalue_7 (`PrimitiveComponent.CreateDynamicMaterialInstance` (`self.MidiFighter_Circle_035`) 1 null "None"))
      (set `self.07` _returnvalue_7))
    (:`then_7`
      (bind _returnvalue_8 (`PrimitiveComponent.CreateDynamicMaterialInstance` (`self.MidiFighter_Circle_029`) 1 null "None"))
      (set `self.08` _returnvalue_8))
    (:`then_8`
      (bind _returnvalue_9 (`PrimitiveComponent.CreateDynamicMaterialInstance` (`self.MidiFighter_Circle_009`) 1 null "None"))
      (set `self.09` _returnvalue_9))
    (:`then_9`
      (bind _returnvalue_10 (`PrimitiveComponent.CreateDynamicMaterialInstance` (`self.MidiFighter_Circle_008`) 1 null "None"))
      (set `self.10` _returnvalue_10))
    (:`then_10`
      (bind _returnvalue_11 (`PrimitiveComponent.CreateDynamicMaterialInstance` (`self.MidiFighter_Circle_021`) 1 null "None"))
      (set `self.11` _returnvalue_11))
    (:`then_11`
      (bind _returnvalue_12 (`PrimitiveComponent.CreateDynamicMaterialInstance` (`self.MidiFighter_Circle_032`) 1 null "None"))
      (set `self.12` _returnvalue_12))
    (:`then_12`
      (bind _returnvalue_13 (`PrimitiveComponent.CreateDynamicMaterialInstance` (`self.MidiFighter_Circle_017`) 1 null "None"))
      (set `self.13` _returnvalue_13))
    (:`then_13`
      (bind _returnvalue_14 (`PrimitiveComponent.CreateDynamicMaterialInstance` (`self.MidiFighter_Circle_057`) 1 null "None"))
      (set `self.14` _returnvalue_14))
    (:`then_14`
      (bind _returnvalue_15 (`PrimitiveComponent.CreateDynamicMaterialInstance` (`self.MidiFighter_Circle_062`) 1 null "None"))
      (set `self.15` _returnvalue_15))
    (:`then_15`
      (bind _returnvalue_16 (`PrimitiveComponent.CreateDynamicMaterialInstance` (`self.MidiFighter_Circle_050`) 1 null "None"))
      (set `self.16` _returnvalue_16))
    (:`then_16`
      (bind _returnvalue_17 (`PrimitiveComponent.CreateDynamicMaterialInstance` (`self.MidiFighter_Circle_039`) 1 null "None"))
      (set `self.17` _returnvalue_17))
    (:`then_17`
      (bind _returnvalue_18 (`PrimitiveComponent.CreateDynamicMaterialInstance` (`self.MidiFighter_Circle_013`) 1 null "None"))
      (set `self.18` _returnvalue_18))
    (:`then_18`
      (bind _returnvalue_19 (`PrimitiveComponent.CreateDynamicMaterialInstance` (`self.MidiFighter_Circle_059`) 1 null "None"))
      (set `self.19` _returnvalue_19))
    (:`then_19`
      (bind _returnvalue_20 (`PrimitiveComponent.CreateDynamicMaterialInstance` (`self.MidiFighter_Circle_064`) 1 null "None"))
      (set `self.20` _returnvalue_20))
    (:`then_20`
      (bind _returnvalue_21 (`PrimitiveComponent.CreateDynamicMaterialInstance` (`self.MidiFighter_Circle_047`) 1 null "None"))
      (set `self.21` _returnvalue_21))
    (:`then_21`
      (bind _returnvalue_22 (`PrimitiveComponent.CreateDynamicMaterialInstance` (`self.MidiFighter_Circle_065`) 1 null "None"))
      (set `self.22` _returnvalue_22))
    (:`then_22`
      (bind _returnvalue_23 (`PrimitiveComponent.CreateDynamicMaterialInstance` (`self.MidiFighter_Circle_023`) 1 null "None"))
      (set `self.23` _returnvalue_23))
    (:`then_23`
      (bind _returnvalue_24 (`PrimitiveComponent.CreateDynamicMaterialInstance` (`self.MidiFighter_Circle_012`) 1 null "None"))
      (set `self.24` _returnvalue_24))
    (:`then_24`
      (bind _returnvalue_25 (`PrimitiveComponent.CreateDynamicMaterialInstance` (`self.MidiFighter_Circle_019`) 1 null "None"))
      (set `self.25` _returnvalue_25))
    (:`then_25`
      (bind _returnvalue_26 (`PrimitiveComponent.CreateDynamicMaterialInstance` (`self.MidiFighter_Circle_031`) 1 null "None"))
      (set `self.26` _returnvalue_26))
    (:`then_26`
      (bind _returnvalue_27 (`PrimitiveComponent.CreateDynamicMaterialInstance` (`self.MidiFighter_Circle_020`) 1 null "None"))
      (set `self.27` _returnvalue_27))
    (:`then_27`
      (bind _returnvalue_28 (`PrimitiveComponent.CreateDynamicMaterialInstance` (`self.MidiFighter_Circle_061`) 1 null "None"))
      (set `self.28` _returnvalue_28))
    (:`then_28`
      (bind _returnvalue_29 (`PrimitiveComponent.CreateDynamicMaterialInstance` (`self.MidiFighter_Circle_066`) 1 null "None"))
      (set `self.29` _returnvalue_29))
    (:`then_29`
      (bind _returnvalue_30 (`PrimitiveComponent.CreateDynamicMaterialInstance` (`self.MidiFighter_Circle_038`) 1 null "None"))
      (set `self.30` _returnvalue_30))
    (:`then_30`
      (bind _returnvalue_31 (`PrimitiveComponent.CreateDynamicMaterialInstance` (`self.MidiFighter_Circle_053`) 1 null "None"))
      (set `self.31` _returnvalue_31))
    (:`then_31`
      (bind _returnvalue_32 (`PrimitiveComponent.CreateDynamicMaterialInstance` (`self.MidiFighter_Circle_049`) 1 null "None"))
      (set `self.32` _returnvalue_32))))